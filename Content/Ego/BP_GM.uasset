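; BP_GM, apparently a game mode, procedurally populates the world around the player with enemies and resources.
; BeginPlay spawns an initial batch of both, then a looping timer keeps adding BP_Enemy actors, each given its default controller.
; Spawn points use random direction and distance from the player pawn at fixed heights, with resources ranging farther out.
; A second looping timer has no visible target event.
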(event `self.ReceiveBeginPlay`
  (`self.Spawn Enemies Procedurally`)
  (`KismetSystemLibrary.K2_SetTimerDelegate` (delegate `SpawnEnemyProcedurally`) 2.0 true)
  (`KismetSystemLibrary.K2_SetTimerDelegate` (`|CreateDelegate` :!event `Spawn Resources Procedurally`) 4.0 true)
  (for _ (range 11)
    (`self.Spawn Resources Procedurally`)))

(event `SpawnEnemyProcedurally`
  (bind _returnvalue (`GameplayStatics.GetPlayerPawn` 0))
  (bind (_returnvalue_x _returnvalue_y) (`KismetMathLibrary.BreakVector` (+ (`self.K2_GetActorLocation` _returnvalue) (* (`KismetMathLibrary.RandomUnitVector`) (`KismetMathLibrary.RandomFloatInRange` 1000.0 6000.0)))))
  (if (`KismetSystemLibrary.IsValid` _returnvalue) :!label _label
    (bind _returnvalue_2 (`|SpawnActorFromClass` "/Game/Ego/BP_Enemy.BP_Enemy_C" (`KismetMathLibrary.MakeTransform` (`KismetMathLibrary.MakeVector` _returnvalue_x _returnvalue_y 250.0)) "Undefined" "OverrideRootScale" null null))
    (if (`KismetSystemLibrary.IsValid` _returnvalue_2)
      (`Pawn.SpawnDefaultController` _returnvalue_2))))

(event `Spawn Enemies Procedurally`
  (for _ (range 11)
    (goto _label)))

(event `Spawn Resources Procedurally`
  (bind _returnvalue (`GameplayStatics.GetPlayerPawn` 0))
  (bind (_returnvalue_x _returnvalue_y) (`KismetMathLibrary.BreakVector` (+ (`self.K2_GetActorLocation` _returnvalue) (* (`KismetMathLibrary.RandomUnitVector`) (`KismetMathLibrary.RandomFloatInRange` 2000.0 8000.0)))))
  (if (`KismetSystemLibrary.IsValid` _returnvalue)
    (`|SpawnActorFromClass` "/Game/Ego/BP_ProceduralResource.BP_ProceduralResource_C" (`KismetMathLibrary.MakeTransform` (`KismetMathLibrary.MakeVector` _returnvalue_x _returnvalue_y 150.0)) "Undefined" "OverrideRootScale" null null)))

(fn `UserConstructionScript`)