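; Procedural resource actor that spawns a small randomized cluster of resource mesh instances around its own location on BeginPlay.
; ProcedurallySpawnRes takes a requested count, falling back to a random count when it is below one, as it is on BeginPlay.
; Each piece is added to ResourceISM in world space with random offset, rotation and non-uniform scale, avoiding separate actors per piece.
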(event `self.ReceiveBeginPlay`
  (`self.ProcedurallySpawnRes` -1))

(fn `ProcedurallySpawnRes`
  (params (SpecificNumRes :type Integer :default -1))
  (locals (`Specific Num Res L` :type Integer :default -1))
  (if (< SpecificNumRes 1)
    (set `local.Specific Num Res L` (`KismetMathLibrary.RandomIntegerInRange` 10 30))
    (else
      (set `local.Specific Num Res L` SpecificNumRes)))
  (for _ (range (+ (`local.Specific Num Res L`) 1))
    (`InstancedStaticMeshComponent.AddInstanceWorldSpace` (`self.ResourceISM`) (`KismetMathLibrary.MakeTransform` (`KismetMathLibrary.MakeVector` (+ (.x (`self.K2_GetActorLocation`)) (`KismetMathLibrary.RandomFloatInRange` -50.0 60.0)) (+ (.y (`self.K2_GetActorLocation`)) (`KismetMathLibrary.RandomFloatInRange` -50.0 60.0)) (+ (.z (`self.K2_GetActorLocation`)) (`KismetMathLibrary.RandomFloatInRange` 0.0 30.0))) (`KismetMathLibrary.RandomRotator` true) (`KismetMathLibrary.MakeVector` (`KismetMathLibrary.RandomFloatInRange` 0.1 0.3) (`KismetMathLibrary.RandomFloatInRange` 0.1 0.3) (`KismetMathLibrary.RandomFloatInRange` 0.1 0.3))))))

(fn `UserConstructionScript`)