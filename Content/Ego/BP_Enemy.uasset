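; BP_Enemy is an enemy that picks between attacking and fleeing when it first spots the player's BP_EgoCharacter.
; PawnSensing stores the target, then a sphere overlap counts nearby BP_Enemy actors: more than two selects attack, otherwise flight.
; AIAttack and AIRunAway are empty stubs, and the move-to-target code is disconnected.
; A BP_EgoCharacter overlapping the Cube component is destroyed.
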(event `self.ReceiveTick`
  (params (DeltaSeconds :type "Float (single-precision)")))

(event `self.PawnSensing.OnHearNoise`
  (params (Instigator :type "Pawn Object Reference") (Location :type "Vector Structure (by ref)") (Volume :type "Float (single-precision)")))

(event `self.PawnSensing.OnSeePawn`
  (params (Pawn :type "Pawn Object Reference"))
  (bind _asthird_person_character (cast `/Game/ThirdPersonCPP/Blueprints/BP_EgoCharacter` Pawn))
  (if (`|EnumEquality` (`self.EnemyState`) "NewEnumerator0")
    (set `self.Target` _asthird_person_character)
    (bind _outactors (`self.Check Friendlies Around`))
    (if (> (`KismetArrayLibrary.Array_Length` _outactors) 2)
      (set `self.EnemyState` "NewEnumerator1")
      (`self.AI_Attack`)
      (else
        (set `self.EnemyState` "NewEnumerator2")
        (`self.AI_RunAway`)))))

(event `self.Cube.OnComponentBeginOverlap`
  (params (OverlappedComponent :type "PrimitiveComponent Object Reference") (OtherActor :type "Actor Object Reference") (OtherComp :type "PrimitiveComponent Object Reference") (OtherBodyIndex :type Integer) (bFromSweep :type Boolean) (SweepResult :type "HitResult Structure (by ref)"))
  (bind _asthird_person_character (cast `/Game/ThirdPersonCPP/Blueprints/BP_EgoCharacter` OtherActor))
  (`self.K2_DestroyActor` _asthird_person_character))

(fn `AI_Attack`)

(fn `AI_RunAway`)

(fn `Check Friendlies Around`
  (returns (OutActors :type "Array of Actor Object Reference"))
  (bind _outactors (`KismetSystemLibrary.SphereOverlapActors` (`self.K2_GetActorLocation`) 1000.0 (`|MakeArray` "ObjectTypeQuery2" :!type "EObjectTypeQuery Enum") "BP_Enemy_C"))
  (return _outactors))

(fn `UserConstructionScript`)