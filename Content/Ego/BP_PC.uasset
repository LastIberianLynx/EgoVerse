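; Player controller that maps debug-style keyboard and mouse input to actions on the possessed BP_EgoCharacter.
; On BeginPlay it casts the controlled pawn and caches the character reference once.
; Input events call straight into that character for hair changes, adding a belt mesh, attacking, gathering resources and equipping with a resource.
; Several calls pass hardcoded test arguments, and the handlers do not check the cached reference.
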(event `self.ReceiveBeginPlay`
  (bind _asthird_person_character (cast `/Game/ThirdPersonCPP/Blueprints/BP_EgoCharacter` (`self.K2_GetPawn`)))
  (set `self.As Third Person Character` _asthird_person_character))

(event `Key|One`
  (params (Key :type "Key Structure"))
  (:`Released`
    (`/Game/ThirdPersonCPP/Blueprints/BP_EgoCharacter.ChangeHair` (`self.As Third Person Character`))))

(event `Key|Two`
  (params (Key :type "Key Structure"))
  (:`Released`
    (`/Game/ThirdPersonCPP/Blueprints/BP_EgoCharacter.ChangeHairSpecificColor` (`self.As Third Person Character`) (make `Color` 0 255 255 255))))

(event `Key|Three`
  (params (Key :type "Key Structure"))
  (:`Released`
    (`/Game/ThirdPersonCPP/Blueprints/BP_EgoCharacter.Add Item` (`self.As Third Person Character`) "/Game/Adventures_woman/Mesh/Adventures_woman/Mesh_UE4/Separate/SK_UE4_Adventures_woman_Belt_01.SK_UE4_Adventures_woman_Belt_01" null)))

(event `Key|LeftMouseButton`
  (params (Key :type "Key Structure"))
  (:`Pressed`
    (`/Game/ThirdPersonCPP/Blueprints/BP_EgoCharacter.Attack` (`self.As Third Person Character`) (0.0 0.0 0.0))))

(event `Key|F`
  (params (Key :type "Key Structure"))
  (:`Released`
    (`/Game/ThirdPersonCPP/Blueprints/BP_EgoCharacter.GatherResource` (`self.As Third Person Character`))))

(event `Key|MouseScrollDown`
  (params (Key :type "Key Structure"))
  (:`Pressed`
    (`/Game/ThirdPersonCPP/Blueprints/BP_EgoCharacter.Equip with Resource2` (`self.As Third Person Character`))))

(fn `UserConstructionScript`)