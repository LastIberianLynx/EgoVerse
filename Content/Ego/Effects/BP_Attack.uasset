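; BP_Attack is a fire projectile actor that destroys what it hits, sparing ThirdPersonCharacter.
; On BeginPlay it yaws its Sphere to Direction, spawns a dash-fire Niagara effect and starts a self-destruct timer.
; Tick moves only the Sphere forward via constant-speed interpolation, without sweeping.
; On Sphere overlap with any other actor, it prints that actor's name, spawns a blink-fire effect and destroys both actors.
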(event `self.ReceiveBeginPlay`
  (bind (_direction_roll _direction_pitch _direction_yaw) (`KismetMathLibrary.BreakRotator` (`self.Direction`)))
  (bind (_direction_roll_2 _direction_pitch_2 _direction_yaw_2) (`KismetMathLibrary.BreakRotator` (`self.Direction`)))
  (`SceneComponent.K2_SetWorldRotation` (`self.Sphere`) (`KismetMathLibrary.MakeRotator` 0.0 0.0 _direction_yaw_2) false false)
  (`NiagaraFunctionLibrary.SpawnSystemAtLocation` "/Game/BlinkAndDashVFX/VFX_Niagara/NS_Dash_Fire.NS_Dash_Fire" (`self.K2_GetActorLocation`) (`KismetMathLibrary.MakeRotator` 0.0 0.0 _direction_yaw))
  (`self.SetActorTickEnabled` true)
  (`KismetSystemLibrary.K2_SetTimerDelegate` (delegate `Destroy`) 4.0))

(event `Destroy`
  (`self.K2_DestroyActor`))

(event `self.ReceiveTick`
  (params (DeltaSeconds :type "Float (single-precision)"))
  (bind _sphere (`self.Sphere`))
  (bind _returnvalue (`SceneComponent.K2_GetComponentLocation` _sphere))
  (`SceneComponent.K2_SetWorldLocation` _sphere (`KismetMathLibrary.VInterpTo_Constant` _returnvalue (+ _returnvalue (* (`SceneComponent.GetForwardVector` _sphere) 100.0)) DeltaSeconds 3000.0) false false))

(event `self.Sphere.OnComponentBeginOverlap`
  (params (OverlappedComponent :type "PrimitiveComponent Object Reference") (OtherActor :type "Actor Object Reference") (OtherComp :type "PrimitiveComponent Object Reference") (OtherBodyIndex :type Integer) (bFromSweep :type Boolean) (SweepResult :type "HitResult Structure (by ref)"))
  (cast `/Game/ThirdPersonCPP/Blueprints/ThirdPersonCharacter` OtherActor
    (:`CastFailed`
      (`KismetSystemLibrary.PrintString` (`KismetSystemLibrary.GetDisplayName` OtherActor))
      (`NiagaraFunctionLibrary.SpawnSystemAtLocation` "/Game/BlinkAndDashVFX/VFX_Niagara/NS_Blink_Fire.NS_Blink_Fire" (`SceneComponent.K2_GetComponentLocation` (`self.Sphere`)) (`KismetMathLibrary.MakeRotator` 0.0))
      (`self.K2_DestroyActor`)
      (`self.K2_DestroyActor` OtherActor))))

(fn `UserConstructionScript`)